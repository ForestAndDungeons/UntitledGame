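; BP_Enemy is an enemy that relays AI perception updates to its AI controller's Blackboard.
; On a successful sense, it casts its controller to BP_AI_Controller, writes the Target key with no object supplied and sets IsTargetInSight true.
; On a failed sense, it sets IsTargetInSight false through that cast result without casting again.
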(event OnTargetPerceptionUpdated(AIPerception)
  (params (Actor :type Actor%20Object%20Reference) (Stimulus :type AI%20Stimulus%20Structure))
  (if (.bSuccessfullySensed (Utilities|Struct|BreakAIStimulus Stimulus))
    (bind _asbp_ai_controller (Utilities|Casting|CastToBP_AI_Controller (Pawn|GetController)))
    (AI|Components|Blackboard|SetValueasObject (Variables|/Script/AIModule.AIController|GetBlackboard _asbp_ai_controller) (Utilities|Name|MakeLiteralName "Target") 0)
    (AI|Components|Blackboard|SetValueasBool (Variables|/Script/AIModule.AIController|GetBlackboard _asbp_ai_controller) (Utilities|Name|MakeLiteralName "IsTargetInSight") true)
    (else
      (AI|Components|Blackboard|SetValueasBool (Variables|/Script/AIModule.AIController|GetBlackboard _asbp_ai_controller) (Utilities|Name|MakeLiteralName "IsTargetInSight") false))))

(event EventBeginPlay)

(event Collision|EventActorBeginOverlap
  (params (OtherActor :type Actor%20Object%20Reference)))

(event EventTick
  (params (DeltaSeconds :type Float%20%28single-precision%29)))

(fn ConstructionScript)