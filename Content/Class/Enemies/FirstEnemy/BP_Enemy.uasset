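; BP_Enemy is an enemy character that periodically attacks the player in front of it.
; On BeginPlay it loads mesh, damage, range, attack rate and speed from DT_EnemiesData, using its class display name as the row key.
; A looping timer sphere-traces forward for pawns, then plays a shotgun montage and applies damage to a hit BP_ThirdPersonCharacter.
; Perception logic for setting AI Blackboard target keys is present but never runs.
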(event Custom|AttackPlayer
  (bind _returnvalue (Transformation|GetActorLocation))
  (bind (_outhit _returnvalue_2) (Collision|SphereTraceForObjects _returnvalue (+ _returnvalue (* (Math|Vector|GetForwardVector (Transformation|GetActorRotation)) (Variables|Default|GetAttackRange))) 0.0 (Utilities|Array|MakeArray "ObjectTypeQuery3") false 0 "None"))
  (if _returnvalue_2
    (Utilities|Casting|CastToBP_ThirdPersonCharacter (.HitActor (Collision|BreakHitResult _outhit)))
    (Animation|PlayAnimMontage "/Game/Class/Enemies/EnemyAnimator/Fire_Shotgun_Hip1_Montage.Fire_Shotgun_Hip1_Montage" 1.0 "None")
    (Game|Damage|ApplyDamage (.HitActor (Collision|BreakHitResult _outhit)) (Variables|Default|GetDamage) 0 0)))

(event EventBeginPlay
  (CallFunction|LoadEnemyValue)
  (if true
    (Variables|/Script/Engine.CharacterMovementComponent|SetMaxWalkSpeed (Variables|Character|GetCharacterMovement) (Variables|Default|GetSpeedMovement))
    (CallFunction|AttackPlayer)
    (Utilities|Time|SetTimerbyEvent (delegate Custom|AttackPlayer) (Variables|Default|GetAttackRate) true)))

(event Collision|EventActorBeginOverlap
  (params (OtherActor :type Actor%20Object%20Reference)))

(event EventTick
  (params (DeltaSeconds :type Float%20%28single-precision%29)))

(fn ConstructionScript)

(fn LoadEnemyValue
  (bind _returnvalue (Utilities|GetDataTableRow "/Game/Class/Enemies/DataTable/DT_EnemiesData.DT_EnemiesData" (Utilities|String|StringToName (Utilities|GetClassDisplayName (Utilities|GetClass self))))
    (:then
      (Class|SkinnedMeshComponent|SetSkeletalMesh (Variables|Character|GetMesh) (.Mesh (Utilities|Struct|BreakFEnemyData _returnvalue)) true)
      (Variables|Default|SetDamage (.Damage (Utilities|Struct|BreakFEnemyData _returnvalue)))
      (Variables|Default|SetAttackRange (.AttackRange (Utilities|Struct|BreakFEnemyData _returnvalue)))
      (Variables|Default|SetAttackRate (.AttackRate (Utilities|Struct|BreakFEnemyData _returnvalue)))
      (Variables|Default|SetSpeedMovement (.SpeedMovement (Utilities|Struct|BreakFEnemyData _returnvalue)))
      (return))))