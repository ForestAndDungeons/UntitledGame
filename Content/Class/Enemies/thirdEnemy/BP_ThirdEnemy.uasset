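; BP_ThirdEnemy is a ranged enemy that fires projectiles at the player character.
; On BeginPlay it loads mesh, scale, speed and attack stats from DT_EnemiesData, using its class display name as the row key.
; ShootEnemy turns it toward Target, plays a fire animation, waits AttackRate, then plays a sound and spawns a BP_FirstPersonProjectile at ShootPosition, recording itself as the projectile's spawner.
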(event Custom|ShootEnemy
  (bind _asbp_third_person_character (Utilities|Casting|CastToBP_ThirdPersonCharacter (Variables|Default|GetTarget)))
  (Transformation|SetActorRotation (Math|Rotator|FindLookatRotation (Transformation|GetActorLocation) (Transformation|GetActorLocation _asbp_third_person_character)))
  (Components|Animation|PlayAnimation (Variables|Character|GetMesh) "/Game/Class/Enemies/EnemyAnimator/Fire_Shotgun_Hip1.Fire_Shotgun_Hip1" false)
  (Utilities|FlowControl|Delay (Variables|Default|GetAttackRate))
  (Audio|PlaySoundatLocation "/Game/Class/Sounds/arrow.arrow" (Transformation|GetActorLocation) "0, 0, 0" 1.0 1.0 0.0 0 0 0 0)
  (bind _returnvalue (Game|SpawnActorfromClass "/Game/FirstPerson/Blueprints/BP_FirstPersonProjectile.BP_FirstPersonProjectile_C" (Transformation|GetWorldTransform (Variables|Default|GetShootPosition)) "Undefined" 0 0))
  (Variables|/Game/FirstPerson/Blueprints/BP_FirstPersonProjectile.BP_FirstPersonProjectile_C|SetMyActorSpawn _returnvalue self))

(event EventBeginPlay
  (CallFunction|LoadEnemyValue)
  (if true
    (Transformation|SetRelativeScale3D (Variables|Character|GetMesh) (Math|Conversions|ToVector(Float) (Variables|Default|GetMeshScale)))
    (Variables|/Script/Engine.CharacterMovementComponent|SetMaxWalkSpeed (Variables|Character|GetCharacterMovement) (Variables|Default|GetSpeedMovement))
    (Components|Animation|PlayAnimation (Variables|Character|GetMesh) "/Game/Class/Enemies/EnemyAnimator/Crouch_Idle_Rifle_Ironsights.Crouch_Idle_Rifle_Ironsights" false)))

(event Collision|EventActorBeginOverlap
  (params (OtherActor :type Actor%20Object%20Reference)))

(event EventTick
  (params (DeltaSeconds :type Float%20%28single-precision%29)))

(fn ConstructionScript)

(fn LoadEnemyValue
  (bind _returnvalue (Utilities|GetDataTableRow "/Game/Class/Enemies/DataTable/DT_EnemiesData.DT_EnemiesData" (Utilities|String|StringToName (Utilities|GetClassDisplayName (Utilities|GetClass self))))
    (:then
      (Class|SkinnedMeshComponent|SetSkeletalMesh (Variables|Character|GetMesh) (.Mesh (Utilities|Struct|BreakFEnemyData _returnvalue)) true)
      (Variables|Default|SetDamage (.Damage (Utilities|Struct|BreakFEnemyData _returnvalue)))
      (Variables|Default|SetAttackRange (.AttackRange (Utilities|Struct|BreakFEnemyData _returnvalue)))
      (Variables|Default|SetAttackRate (.AttackRate (Utilities|Struct|BreakFEnemyData _returnvalue)))
      (Variables|Default|SetSpeedMovement (.SpeedMovement (Utilities|Struct|BreakFEnemyData _returnvalue)))
      (Variables|Default|SetMeshScale (.MeshScale (Utilities|Struct|BreakFEnemyData _returnvalue)))
      (return))))