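; BP_Lever is a lever actor that opens a linked BP_Door and shows an interact prompt when the player is near.
; The WidgetTrigger overlap events toggle the Interact component's visibility for BP_FirstPersonCharacter, and BeginPlay hides it.
; InteractToPlayer passes Door to MoveDoor, which casts it to BP_Door and calls its MoveDoor with a fixed upward vector.
; Nothing in this event graph triggers InteractToPlayer, as its only call here is unwired.
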(event OnComponentBeginOverlap(WidgetTrigger)
  (params (OverlappedComponent :type Primitive%20Component%20Object%20Reference) (OtherActor :type Actor%20Object%20Reference) (OtherComp :type Primitive%20Component%20Object%20Reference) (OtherBodyIndex :type Integer) (bFromSweep :type Boolean) (SweepResult :type Hit%20Result%20Structure%20%28by%20ref%29))
  (Utilities|Casting|CastToBP_FirstPersonCharacter OtherActor)
  (Rendering|SetVisibility (Variables|Default|GetInteract) true false))

(event OnComponentEndOverlap(WidgetTrigger)
  (params (OverlappedComponent :type Primitive%20Component%20Object%20Reference) (OtherActor :type Actor%20Object%20Reference) (OtherComp :type Primitive%20Component%20Object%20Reference) (OtherBodyIndex :type Integer))
  (Utilities|Casting|CastToBP_FirstPersonCharacter OtherActor)
  (Rendering|SetVisibility (Variables|Default|GetInteract) false false))

(event EventBeginPlay
  (Rendering|SetVisibility (Variables|Default|GetInteract) false false))

(event Collision|EventActorBeginOverlap
  (params (OtherActor :type Actor%20Object%20Reference)))

(event EventTick
  (params (DeltaSeconds :type Float%20%28single-precision%29)))

(fn ConstructionScript)

(fn MoveDoor
  (params (DoorToActive :type Actor%20Object%20Reference))
  (bind _asbp_door (Utilities|Casting|CastToBP_Door DoorToActive))
  (Default|MoveDoor _asbp_door "0.000000,0.000000,400.000000"))

(fn InteracttoPlayer
  (CallFunction|MoveDoor (Variables|Default|GetDoor)))