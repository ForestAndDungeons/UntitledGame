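; BPC_HPSystem is an actor component that tracks the player character's health and handles defeat.
; On BeginPlay it caches the owning BP_ThirdPersonCharacter and fills HP to max if the owner implements BPI_HPSystem.
; ChangeHealth clamps the new value, updates the HUD health bar, prints it, then runs IsDead.
; At zero HP, IsDead sends DeadMessage to the owner and, after a short delay, opens the Defeat level.
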(event Custom|IsDead
  (if (<= (Variables|Default|GetCurrentHP) 0.0)
    (Class|BPIHPSystem|Dead(Message) (Components|GetOwner))
    (Utilities|FlowControl|Delay 1.5)
    (Game|OpenLevel(byObjectReference) "/Game/Class/Defeat.Defeat")))

(event Custom|ChangeHealth
  (params (HPChange :type Float%20%28double-precision%29))
  (bind _output_get (Variables|Default|SetCurrentHP (Math|Float|Clamp(Float) (+ (Variables|Default|GetCurrentHP) HPChange) 0.0 (Variables|Default|GetMaxHP))))
  (Progress|SetPercent (Variables|/Game/Class/WP_Health.WP_Health_C|GetHealthBar (Variables|/Game/ThirdPerson/Blueprints/BP_ThirdPersonCharacter.BP_ThirdPersonCharacter_C|GetHUD%20widget (Variables|Default|GetPlayerCharacter))) (/ _output_get (Variables|Default|GetMaxHP)))
  (Development|PrintString (Utilities|String|ToString(Text) (Utilities|Text|FormatText "HP:  {HP}" (Variables|Default|GetCurrentHP))))
  (CallFunction|IsDead))

(event EventBeginPlay
  (bind _returnvalue (Components|GetOwner))
  (bind _asbp_third_person_character (Utilities|Casting|CastToBP_ThirdPersonCharacter _returnvalue))
  (Variables|Default|SetPlayerCharacter _asbp_third_person_character)
  (if (Utilities|DoesObjectImplementInterface _returnvalue "/Game/Class/ActorCompónent/BPI_HPSystem.BPI_HPSystem_C")
    (Variables|Default|SetCurrentHP (Variables|Default|GetMaxHP))))

(event EventTick
  (params (DeltaSeconds :type Float%20%28single-precision%29)))