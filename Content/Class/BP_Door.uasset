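; BP_Door is a door actor with unfinished movement logic, storing its start location and a point 400 units above at BeginPlay.
; Tick re-sets a looping 1 ms StartTimer every frame, which decrements a counter and teleports the door to world origin at zero.
; MoveDoor applies an offset only if it lands exactly on the raised point, otherwise restoring the start location, but its only call never runs.
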(event EventBeginPlay
  (Variables|Default|SetDefaultPosition (Transformation|GetActorLocation))
  (Variables|Default|SetPositionMax (+ (Transformation|GetActorLocation) "0,0,400.000000")))

(event Collision|EventActorBeginOverlap
  (params (OtherActor :type Actor%20Object%20Reference)))

(event EventTick
  (params (DeltaSeconds :type Float%20%28single-precision%29))
  (Utilities|Time|SetTimerbyFunctionName 0 "StartTimer" 0.001 true))

(fn ConstructionScript)

(fn MoveDoor
  (params (OffSet :type Vector))
  (bind _returnvalue (Transformation|GetActorLocation))
  (bind _returnvalue_2 (+ _returnvalue OffSet))
  (if (Class|KismetMathLibrary|EqualExactlyVectorVector _returnvalue_2 (Variables|Default|GetPositionMax))
    (Transformation|SetActorLocation _returnvalue_2 false false)
    (return)
    (else
      (Transformation|SetActorLocation (Variables|Default|GetDefaultPosition) false false))))

(fn StartTimer
  (bind _result (Math|Integer|DecrementInt (Variables|Default|Getmiliseconds))
    (:%20%20
      (if (== _result 0)
        (Transformation|SetActorLocation self "0, 0, 0" false false)))))